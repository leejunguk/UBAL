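; BP_MapOut is an overlap trigger that teleports a CustomeVehicle leaving through it to a randomly picked BP_MapOut's OutDirection.
; BeginPlay caches all BP_MapOut actors; overlap stops the vehicle, disables its collision, moves and rotates it, then nudges it forward.
; Each validity, location and rotation lookup rolls its own random index, so targets can differ.
; Collision re-enable is unconnected, and the similar RandomTeleport function is never called here.
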(event `self.ReceiveBeginPlay`
  (bind _outactors (`GameplayStatics.GetAllActorsOfClass` "BP_MapOut_C"))
  (set `self.MapOutList` _outactors))

(event `self.ReceiveActorBeginOverlap`
  (params (OtherActor :type "Actor Object Reference"))
  (bind _mapoutlist (`self.MapOutList`))
  (bind _output (`|GetArrayItem` _mapoutlist (`KismetMathLibrary.RandomIntegerInRange` 0 (`KismetArrayLibrary.Array_LastIndex` _mapoutlist))))
  (bind _outdirection (`/Game/BP_MapOut.OutDirection` _output))
  (bind _ascustome_vehicle (cast `CustomeVehicle` OtherActor))
  (`MovementComponent.StopMovementImmediately` (`WheeledVehicle.VehicleMovement` _ascustome_vehicle))
  (`self.SetActorEnableCollision` _ascustome_vehicle false)
  (`/Engine/EditorBlueprintResources/StandardMacros.IsValid` _output
    (:`Is Valid`
      (`self.K2_SetActorLocation` _ascustome_vehicle (`SceneComponent.K2_GetComponentLocation` _outdirection) false true)
      (`self.K2_SetActorRotation` _ascustome_vehicle (`KismetMathLibrary.FindLookAtRotation` (`SceneComponent.K2_GetComponentLocation` (`WheeledVehicle.Mesh` _ascustome_vehicle)) (`SceneComponent.K2_GetComponentLocation` _outdirection)) true)
      (`CustomeVehicle.OnHandbrakeReleased` _ascustome_vehicle)
      (`CustomeVehicle.MoveForward` _ascustome_vehicle 0.5))))

(event `self.ReceiveActorEndOverlap`
  (params (OtherActor :type "Actor Object Reference")))

(fn `Random Teleport`
  (params (Vehicle :type "CustomeVehicle Object Reference"))
  (bind _mapoutlist (`self.MapOutList`))
  (bind _output (`|GetArrayItem` _mapoutlist (`KismetMathLibrary.RandomIntegerInRange` 0 (`KismetArrayLibrary.Array_LastIndex` _mapoutlist))))
  (`/Engine/EditorBlueprintResources/StandardMacros.IsValid` _output
    (:`Is Valid`
      (bind _asbp_map_out (cast `/Game/BP_MapOut` _output)
        (:`then`
          (`self.K2_SetActorLocation` Vehicle (`SceneComponent.K2_GetComponentLocation` (`/Game/BP_MapOut.OutDirection` _asbp_map_out)) false true)
          (return))
        (:`CastFailed`
          (return))))
    (:`Is Not Valid`
      (return))))

(fn `UserConstructionScript`)