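; AI controller for cars that starts the car behavior tree and sets its blackboard on BeginPlay.
; A LidarTick event line-traces 3000 units along world +X, not the car's forward vector, with debug drawing.
; It zeroes the CustomeVehicle pawn's MoveForward input on a hit and drives full forward otherwise.
; The only LidarTick call in this graph is disconnected, and Tick is empty.
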(event `self.ReceiveBeginPlay`
  (`self.RunBehaviorTree` "/Game/BT_CarAI.BT_CarAI")
  (`self.UseBlackboard` "/Game/BB_Car.BB_Car"))

(event `self.ReceiveTick`
  (params (DeltaSeconds :type "Float (single-precision)")))

(event `LidarTick`
  (bind _returnvalue (`self.K2_GetPawn`))
  (bind (_returnvalue_x _returnvalue_y _returnvalue_z) (`KismetMathLibrary.BreakVector` (`self.K2_GetActorLocation` _returnvalue)))
  (bind (_outhit _returnvalue_2) (`KismetSystemLibrary.LineTraceSingle` :`Start` (`self.K2_GetActorLocation` _returnvalue) :`End` (`KismetMathLibrary.MakeVector` (+ _returnvalue_x 3000.0) _returnvalue_y _returnvalue_z) :`TraceChannel` "TraceTypeQuery2" :`DrawDebugType` "ForDuration"))
  (bind _ascustome_vehicle (cast `CustomeVehicle` _returnvalue))
  (if _returnvalue_2
    (`CustomeVehicle.MoveForward` _ascustome_vehicle 0.0)
    (else
      (`CustomeVehicle.MoveForward` _ascustome_vehicle 1.0))))

(fn `UserConstructionScript`)